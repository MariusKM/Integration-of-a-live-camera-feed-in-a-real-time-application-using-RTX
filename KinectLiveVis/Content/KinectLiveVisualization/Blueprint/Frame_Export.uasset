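; Kinect live-view actor that shows a selected sensor frame type on a plane and exports it through a render target.
; On BeginPlay it initializes the sensor, polls until it is available, scales the plane to the frame's aspect ratio and feeds the frame texture into a dynamic material.
; Every Tick draws that material to the render target and calls export with blank path and file name; Escape uninitializes the sensor.
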(event `self.ReceiveBeginPlay`
  (bind _plane (`self.Plane`))
  (bind _returnvalue (`NeoKinectManager.GetFrameSize` (`self.FrameType`)))
  (bind (_x _y) (break `IntPoint` _returnvalue))
  (`NeoKinectManager.InitSensor`)
  (`KismetSystemLibrary.PrintString` (`KismetStringLibrary.Conv_IntPointToString` _returnvalue))
  (if (`NeoKinectManager.IsKinectAvailable`) :!label _label
    (`|ExecutionSequence`
      (:`then_0`
        (`SceneComponent.SetRelativeScale3D` _plane (`KismetMathLibrary.MakeVector` 1.0 (/ (`KismetMathLibrary.Conv_IntToDouble` _y) (`KismetMathLibrary.Conv_IntToDouble` _x)) 1.0))
        (bind _returnvalue_2 (`PrimitiveComponent.CreateDynamicMaterialInstance` _plane 0 null "None"))
        (bind _returnvalue_3 (`NeoKinectManager.SetUseFrame` (`self.FrameType`) true))
        (`MaterialInstanceDynamic.SetTextureParameterValue` _returnvalue_2 "Texture" _returnvalue_3)
        (bind _returnvalue_4 (`MaterialInstanceDynamic.K2_GetTextureParameterValue` _returnvalue_2 "Texture"))
        (set `Texture.AdjustMinAlpha` 1.0 _returnvalue_4)))
    (else
      (`KismetSystemLibrary.Delay` 0.2)
      (goto _label))))

(event `self.ReceiveTick`
  (params (DeltaSeconds :type "Float (single-precision)"))
  (bind _rendertarget (`self.RenderTarget`))
  (`KismetRenderingLibrary.DrawMaterialToRenderTarget` _rendertarget (stale `self.ReceiveBeginPlay` _returnvalue_2))
  (`KismetRenderingLibrary.ExportRenderTarget` _rendertarget))

(event `Key|Escape`
  (params (Key :type "Key Structure"))
  (:`Pressed`
    (`NeoKinectManager.UninitSensor`)))

(fn `UserConstructionScript`)