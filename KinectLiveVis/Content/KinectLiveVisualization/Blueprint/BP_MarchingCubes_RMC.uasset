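; Actor that builds a marching cubes mesh on a RuntimeMeshComponent from a Niagara grid, with debug single-cell, vertex and wireframe options.
; BeginPlay generates cell corner indices and passes grid settings to Niagara.
; Niagara's particle callback triggers CPU readback of RTTriangles, decoding each color channel into an edge index.
; Vertices sit at edge midpoints on a recomputed grid, and the Update flag stops rebuilds after the first mesh creation.
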(event `self.ReceiveBeginPlay`
  (bind _niagara (`self.Niagara`))
  (`NiagaraComponent.SetNiagaraVariableObject` _niagara "User.BP_Callback" self)
  (`self.Generate Cell Corners` (`self.xSize`) (`self.ySize`) (`self.zSize`))
  (`NiagaraComponent.SetNiagaraVariableInt` _niagara "User.xSize" (`self.xSize`))
  (`NiagaraComponent.SetNiagaraVariableInt` _niagara "User.ySize" (`self.ySize`))
  (`NiagaraComponent.SetNiagaraVariableInt` _niagara "User.zSize" (`self.zSize`))
  (`NiagaraComponent.SetNiagaraVariableVec3` _niagara "User.GridSize" (`self.GridSize`)))

(event `self.ReceiveParticleData`
  (params (Data :type "Array of BasicParticleData Structure (by ref)") (NiagaraSystem :type "NiagaraSystem Object Reference"))
  (bind _rt_triangles (`self.RT_Triangles`))
  (bind _edges (`self.Edges`))
  (if (not (`self.update`))
    (`|ExecutionSequence`
      (:`then_0`
        ;[1 1 1] Clear Array
        (`KismetArrayLibrary.Array_Clear` (`self.FinalVerts`))
        (`KismetArrayLibrary.Array_Clear` (`self.Edges`))
        (`KismetArrayLibrary.Array_Clear` (`self.ParticlePos`))
        (`KismetArrayLibrary.Array_Clear` (`self.ColorsOut`))
        (`KismetArrayLibrary.Array_Clear` (`self.DebugTris`))
        (`KismetArrayLibrary.Array_Clear` (`self.DebugINdex`))
        (for _array_element (`self.Cells`)
          _))
      (:`then_1`
        (`|ExecutionSequence`
          (:`then_0`
            ;[1 1 1] ReadPixelValues
            (for _index (range (`TextureRenderTarget2D.SizeY` _rt_triangles))
              (for _index_2 (range (`TextureRenderTarget2D.SizeX` _rt_triangles))
                (bind _returnvalue (`KismetRenderingLibrary.ReadRenderTargetPixel` _rt_triangles _index_2 _index))
                (`KismetArrayLibrary.Array_Add` (`self.ColorsOut`) _returnvalue))))
          (:`then_1`
            (`KismetSystemLibrary.PrintString` "Hello")
            ;[1 1 1] CovertPixelVals To edge
            (for (_array_element_2 _array_index) (`self.ColorsOut`)
              (`|ExecutionSequence`
                (:`then_0`
                  (bind _edgeindex (`self.ColorToEdge` (`KismetMathLibrary.Conv_ByteToDouble` (`.R` (break `Color` _array_element_2)))))
                  (`KismetArrayLibrary.Array_Add` _edges _edgeindex))
                (:`then_1`
                  (bind _edgeindex_2 (`self.ColorToEdge` (`KismetMathLibrary.Conv_ByteToDouble` (`.G` (break `Color` _array_element_2)))))
                  (`KismetArrayLibrary.Array_Add` _edges _edgeindex_2))
                (:`then_2`
                  (bind _edgeindex_3 (`self.ColorToEdge` (`KismetMathLibrary.Conv_ByteToDouble` (break `Color` _array_element_2))))
                  (`KismetArrayLibrary.Array_Add` _edges _edgeindex_3))
                (:`then_3`
                  (bind _edgeindex_4 (`self.ColorToEdge` (`KismetMathLibrary.Conv_ByteToDouble` (`.A` (break `Color` _array_element_2)))))
                  (`KismetArrayLibrary.Array_Add` _edges _edgeindex_4))
                (:`then_4`))))
          (:`then_2`
            (`self.CacheParticlePos` (`self.xSize`) (`self.ySize`) (`self.zSize`) (`self.GridSize`)))
          (:`then_3`
            ;[1 1 1] Calculate VertexPositions
            (for (_array_element_3 _array_index_2) (`self.Edges`)
              (if (!= _array_element_3 -1)
                (bind (_verta _vertb _currentcellindex) (`self.Get Edge Verts` _array_element_3 _array_index_2))
                (bind _newvert (`self.Calc New Vertex Pos` _verta _vertb _currentcellindex))
                (if (`self.RenderSingle`)
                  (if (== _currentcellindex (`self.Single Cell Index`))
                    (`KismetArrayLibrary.Array_Add` (`self.FinalVerts`) _newvert)
                    (`KismetArrayLibrary.Array_Add` (`self.DebugTris`) _array_element_3))
                  (else
                    (`KismetArrayLibrary.Array_Add` (`self.FinalVerts`) _newvert))))))
          (:`then_4`
            ;[1 1 1] Create Mesh
            (`self.CreateMesh` (`self.FinalVerts`) "/Game/KinectLiveVisualization/Materials/M_ProceduralMesh.M_ProceduralMesh" "/Engine/EngineDebugMaterials/WireframeMaterial.WireframeMaterial" (`self.Wireframe`)))
          (:`then_5`
            ;[1 1 1] DebugVert
            (if (`self.DebugVert`)
              (`self.Debug Vert Pos` (`self.FinalVerts`)))))))))

(fn `CacheParticlePos`
  (params (xSize :type Integer) (ySize :type Integer) (zSize :type Integer) (GridSize :type "Vector Structure"))
  (locals (NumParticles :type Integer) (xCount :type Integer) (yCount :type Integer) (XYZCount :type "Vector Structure") (GridDIm :type "Vector Structure"))
  (bind _xcount (`local.xCount`))
  (bind _ycount (`local.yCount`))
  (set `local.GridDIm` GridSize)
  (set `local.XYZCount` (`KismetMathLibrary.MakeVector` (- (`KismetMathLibrary.Conv_IntToDouble` xSize) 1.0) (- (`KismetMathLibrary.Conv_IntToDouble` ySize) 1.0) (- (`KismetMathLibrary.Conv_IntToDouble` zSize) 1.0)))
  (set `local.xCount` xSize)
  (set `local.yCount` ySize)
  (bind _output_get (set `local.NumParticles` (* xSize ySize zSize)))
  (for _index (range _output_get)
    (bind _returnvalue (/ _index (* _xcount _ycount)))
    (bind _returnvalue_2 (- _index (* (* _returnvalue _xcount) _ycount)))
    (`KismetArrayLibrary.Array_Add` (`self.ParticlePos`) (* (- (`KismetMathLibrary.MakeVector` (`KismetMathLibrary.Conv_IntToDouble` (mod _returnvalue_2 _xcount)) (`KismetMathLibrary.Conv_IntToDouble` (/ _returnvalue_2 _xcount)) (`KismetMathLibrary.Conv_IntToDouble` _returnvalue)) (* (`local.XYZCount`) 0.5)) (/ (`local.GridDIm`) (`local.XYZCount`))))))

(fn `Calc New Vertex Pos`
  (params (VertexA :type "Vector Structure") (VertexB :type "Vector Structure") (CurrentCellIndex :type Integer))
  (returns (NewVert :type "Vector Structure"))
  (bind _returnvalue (/ (+ VertexA VertexB) 2.0))
  (`KismetArrayLibrary.Array_Add` (`.NewVerts_7_0669F2AB41A8F083362D1D925A427AC0` (break `/Game/KinectLiveVisualization/Blueprint/Cell` (`|GetArrayItem` (`self.Cells`) CurrentCellIndex))) _returnvalue)
  (return _returnvalue))

(fn `ColorToEdge`
  (params (ColorVal :type "Float (double-precision)"))
  (returns (EdgeIndex :type Integer))
  (return (- (`KismetMathLibrary.Round` (* (/ ColorVal 255.0) 12.0)) 1)))

(fn `CreateMesh`
  (params (NewVerts :type "Array of Vector Structure") (MeshMat :type "Material Object Reference") (WireMat :type "Material Object Reference") (Wireframe :type Boolean))
  (locals (Triangles :type "Array of Integer"))
  (bind _runtimemeshcomponentstatic (`self.RuntimeMeshComponentStatic`))
  (bind _triangles (`local.Triangles`))
  (bind _runtimemeshcomponentstatic_2 (`self.RuntimeMeshComponentStatic`))
  (for (_ _array_index) NewVerts
    (`KismetArrayLibrary.Array_Add` _triangles _array_index))
  (if (`self.update`)
    (`KismetSystemLibrary.PrintString` "Hello")
    (`RuntimeMeshComponentStatic.UpdateSectionFromComponents` :`self` _runtimemeshcomponentstatic_2 :`Vertices` NewVerts :`Triangles` _triangles)
    (else
      (`RuntimeMeshComponentStatic.CreateSectionFromComponents` :`self` _runtimemeshcomponentstatic_2 :`Vertices` NewVerts :`Triangles` _triangles :`bCreateCollision` false)
      (set `self.update` true)))
  (if Wireframe
    (`PrimitiveComponent.SetMaterial` _runtimemeshcomponentstatic 0 WireMat)
    (else
      (`PrimitiveComponent.SetMaterial` _runtimemeshcomponentstatic 0 MeshMat))))

(fn `Debug Vert Pos`
  (params (NewVerts :type "Array of Vector Structure"))
  (for _array_element NewVerts
    (`KismetSystemLibrary.DrawDebugSphere` (+ (`SceneComponent.K2_GetComponentLocation` (`self.RuntimeMeshComponentStatic`)) _array_element) 10.0 12 (struct :`R` 1.0 :`G` 1.0 :`B` 1.0 :`A` 1.0) 5.0)))

(fn `Edge to Vert Index`
  (params (EdgeIndex :type Integer))
  (returns (VertA :type Integer) (VertB :type Integer))
  (locals (EdgeToVertA :type "Array of Integer") (EdgeToVertB :type "Array of Integer"))
  (return (`|GetArrayItem` (`local.EdgeToVertA`) EdgeIndex) (`|GetArrayItem` (`local.EdgeToVertB`) EdgeIndex)))

(fn `Generate Cell Corners`
  (params (xSize :type Integer) (ySize :type Integer) (zSize :type Integer))
  (locals (numCells :type Integer) (m_xSize :type Integer) (m_ySize :type Integer) (m_zSize :type Integer) (offset_Z :type Integer) (offset_Y :type Integer) (heightOffset :type Integer) (rowSize :type Integer) (planeSize :type Integer) (planeCount :type Integer) (heightCount :type Integer) (rowCount :type Integer) (CellVal :type Integer) (CornerIndex :type "Array of Integer"))
  (bind _m_xsize (`local.m_xSize`))
  (`|ExecutionSequence`
    (:`then_0`
      ;[1 1 1] cache Local Vars
      (`|ExecutionSequence`
        (:`then_0`
          (set `local.m_xSize` (- xSize 1))
          (set `local.m_ySize` (- ySize 1))
          (set `local.m_zSize` (- zSize 1)))
        (:`then_1`
          (set `local.numCells` (* (`local.m_xSize`) (`local.m_ySize`) (`local.m_zSize`))))
        (:`then_2`
          (set `local.offset_Z` xSize)
          (set `local.offset_Y` (* xSize zSize)))
        (:`then_3`
          (set `local.heightOffset` (- (+ xSize zSize) 1)))
        (:`then_4`
          (set `local.rowSize` _m_xsize)
          (set `local.planeSize` (* _m_xsize (`local.m_zSize`))))))
    (:`then_1`
      (for _index (range (`local.numCells`))
        (`|ExecutionSequence`
          (:`then_0`
            (bind _output_get (set `local.planeCount` (`KismetMathLibrary.FFloor` (/ (`KismetMathLibrary.Conv_IntToDouble` _index) (`KismetMathLibrary.Conv_IntToDouble` (`local.planeSize`))))))
            (set `local.heightCount` (* _output_get (`local.heightOffset`)))
            (set `local.rowCount` (`KismetMathLibrary.FFloor` (/ (`KismetMathLibrary.Conv_IntToDouble` (- _index (* (`local.planeCount`) (`local.planeSize`)))) (`KismetMathLibrary.Conv_IntToDouble` (`local.rowSize`))))))
          (:`then_1`
            (set `local.CellVal` (+ (+ _index (`local.rowCount`)) (`local.heightCount`))))
          (:`then_2`
            (for _index_2 (range 2)
              (for _index_3 (range 2)
                (for _index_4 (range 2)
                  (`KismetArrayLibrary.Array_Add` (`local.CornerIndex`) (`KismetSystemLibrary.MakeLiteralInt` (+ (+ (+ (`local.CellVal`) (* _index_2 (`local.offset_Y`))) (* _index_3 (`local.offset_Z`))) _index_4)))))))
          (:`then_3`
            (`KismetArrayLibrary.Array_Add` (`self.Cells`) (make `/Game/KinectLiveVisualization/Blueprint/Cell` (`local.CornerIndex`)))
            (`KismetArrayLibrary.Array_Clear` (`local.CornerIndex`))))))))

(fn `Get Edge Verts`
  (params (EdgeIndex :type Integer) (Index :type Integer))
  (returns (VertA :type "Vector Structure") (VertB :type "Vector Structure") (CurrentCellIndex :type Integer))
  (bind (_verta _vertb) (`self.Edge to Vert Index` EdgeIndex))
  (bind _debugindex (`self.DebugINdex`))
  (bind _particlepos (`self.ParticlePos`))
  (bind _returnvalue (`KismetMathLibrary.FFloor` (/ (`KismetMathLibrary.Conv_IntToDouble` Index) 16.0)))
  (bind _cornerindex (break `/Game/KinectLiveVisualization/Blueprint/Cell` (`|GetArrayItem` (`self.Cells`) _returnvalue)))
  (bind _output (`|GetArrayItem` _cornerindex _verta))
  (bind _output_2 (`|GetArrayItem` _cornerindex _vertb))
  (if (== _returnvalue (`self.Single Cell Index`))
    (`KismetArrayLibrary.Array_Add` _debugindex _output)
    (`KismetArrayLibrary.Array_Add` _debugindex _output_2))
  (return (`|GetArrayItem` _particlepos _output) (`|GetArrayItem` _particlepos _output_2) _returnvalue))

(fn `UserConstructionScript`)